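; BP_Door is a door actor that swings open once the player has collected all items.
; On BeginPlay it casts and caches BP_ThirdPersonGameMode, printing an error if the cast fails.
; Each Tick it polls the game mode's AllItemsCollected flag, then sets IsOpened and adds yaw to the Door component at OpeningSpeed, scaled by delta time, until it reaches OpenedAngle.
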(event EventBeginPlay
  (CallFunction|InitializeGameModeReference))

(event Collision|EventActorBeginOverlap
  (params (OtherActor :type Actor%20Object%20Reference)))

(event EventTick
  (params (DeltaSeconds :type Float%20%28single-precision%29))
  (if (Variables|/Game/ThirdPerson/Blueprints/BP_ThirdPersonGameMode.BP_ThirdPersonGameMode_C|GetAllItemsCollected (Variables|Default|GetGameModeReference))
    (Variables|Default|SetIsOpened true)
    (if (< (.yaw (Variables|/Script/Engine.SceneComponent|GetRelativeRotation (Variables|Default|GetDoor))) (Variables|Default|GetOpenedAngle))
      (Transformation|AddRelativeRotation (Variables|Default|GetDoor) (Math|Rotator|MakeRotator 0.0 0.0 (* (Utilities|Time|GetWorldDeltaSeconds) (Variables|Default|GetOpeningSpeed))) false false))))

(fn ConstructionScript)

(fn InitializeGameModeReference
  (bind _asbp_third_person_game_mode (Utilities|Casting|CastToBP_ThirdPersonGameMode (Game|GetGameMode))
    (:then
      (Variables|Default|SetGameModeReference _asbp_third_person_game_mode))
    (:CastFailed
      (Development|PrintString "Game mode cast failed!" true true "(R=1.000000,G=0.000000,B=0.000000,A=1.000000)"))))