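; BP_Item is a collectible pickup actor that spins in place until the player character touches it.
; On BeginPlay it caches the third-person game mode, printing an error if the cast fails.
; When a BP_ThirdPersonCharacter overlaps it, it calls the game mode's EventOnItemPickedUp and destroys itself.
; Tick applies a frame-rate-independent local yaw rotation scaled by RotationSpeed.
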(event EventBeginPlay
  (CallFunction|InitializeGameModeReference))

(event Collision|EventActorBeginOverlap
  (params (OtherActor :type Actor%20Object%20Reference))
  (Utilities|Casting|CastToBP_ThirdPersonCharacter OtherActor)
  (Default|EventonItemPickedUp (Variables|Default|GetGameModeReference))
  (Actor|DestroyActor))

(event EventTick
  (params (DeltaSeconds :type Float%20%28single-precision%29))
  (CallFunction|Rotate DeltaSeconds))

(fn ConstructionScript)

(fn InitializeGameModeReference
  (bind _asbp_third_person_game_mode (Utilities|Casting|CastToBP_ThirdPersonGameMode (Game|GetGameMode))
    (:then
      (Variables|Default|SetGameModeReference _asbp_third_person_game_mode))
    (:CastFailed
      (Development|PrintString "Game mode cast failed!" true true "(R=1.000000,G=0.000000,B=0.000000,A=1.000000)"))))

(fn Rotate
  (params (DeltaSeconds :type Float%20%28double-precision%29))
  (Transformation|AddActorLocalRotation (Math|Rotator|MakeRotator 0.0 0.0 (* DeltaSeconds (Variables|Default|GetRotationSpeed))) false false))