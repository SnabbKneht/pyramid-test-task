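; BP_Enemy is a wandering enemy that moves in random horizontal directions and reacts when it bumps into the player.
; A looping one-second timer calls SetNewDirection to pick a new random XY direction, which Tick feeds into AddMovementInput scaled by MovementSpeed.
; Capsule hits against BP_ThirdPersonCharacter call that character's CheckHit, leaving the outcome to the player.
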(event OnComponentHit(CapsuleComponent)
  (params (HitComponent :type Primitive%20Component%20Object%20Reference) (OtherActor :type Actor%20Object%20Reference) (OtherComp :type Primitive%20Component%20Object%20Reference) (NormalImpulse :type Vector :default "0, 0, 0") (Hit :type Hit%20Result%20Structure%20%28by%20ref%29))
  (bind _asbp_third_person_character (Utilities|Casting|CastToBP_ThirdPersonCharacter OtherActor))
  (Default|CheckHit _asbp_third_person_character))

(event EventBeginPlay
  (CallFunction|SetNewDirection)
  (Utilities|Time|SetTimerbyFunctionName 0 "SetNewDirection" 1.0 true))

(event Collision|EventActorBeginOverlap
  (params (OtherActor :type Actor%20Object%20Reference)))

(event EventTick
  (params (DeltaSeconds :type Float%20%28single-precision%29))
  (Pawn|Input|AddMovementInput (Variables|Default|GetCurrentDirection) (Variables|Default|GetMovementSpeed) false))

(fn ConstructionScript)

(fn SetNewDirection
  (Variables|Default|SetCurrentDirection (Math|Vector|MakeVector (Math|Random|RandomFloatinRange -1.0 1.0) (Math|Random|RandomFloatinRange -1.0 1.0) 0.0)))